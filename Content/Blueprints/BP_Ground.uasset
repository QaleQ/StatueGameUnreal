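; BP_Ground is a ground actor that records its horizontal extents as MinX, MaxX, MinY and MaxY variables when play begins.
; BeginPlay feeds the actor bounds' origin and box extent into CalculateBounds and passes its outputs to Setters, which stores them.
; CalculateBounds holds origin plus and minus extent math for X and Y, though those results appear unconnected to its outputs.
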(event EventBeginPlay
  (bind (_origin _boxextent) (Collision|GetActorBounds false false))
  (bind (_maxx _minx _maxy _miny) (|CalculateBounds (.x _origin) (.y _origin) (.x _boxextent) (.y _boxextent)))
  ;[1 0 0] Event BeginPlay
  ;;[1 1 1] Initialize variables
  (|Setters _maxx _minx _maxy _miny))

(fn ConstructionScript)