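; BP_Statue is a collectible statue that periodically teleports while awaiting pickup by the player.
; A Delay on Tick spaces the moves, shortening as the custom game mode's current level rises.
; Player overlap during an active game spawns a replacement statue, notifies the game mode and destroys this one.
; Teleports and spawns both take their transform from GenerateRandomLocation.
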(event Custom|SpawnStatue
  ;[1 1 1] Spawn Statue
  (Game|SpawnActorfromClass "BP_Statue_C" (Utilities|GenerateRandomLocation) "AdjustIfPossibleButAlwaysSpawn" "MultiplyWithRoot" 0 0))

(event EventTick
  (params (DeltaSeconds :type Float%20%28single-precision%29))
  ;[1 1 1] Teleport logic
  (Utilities|FlowControl|Delay (Math|Conversions|ToFloat(Integer) (- 6 (Variables|/Game/ThirdPerson/Blueprints/BP_ThirdPersonGameMode.BP_ThirdPersonGameMode_C|GetLevelCurrent (Variables|Default|GetCustomGameMode)))))
  (Transformation|SetActorTransform (Utilities|GenerateRandomLocation)))

(event EventBeginPlay
  ;[1 0 0] Event BeginPlay
  ;;[1 1 1] Set variables
  (bind _asbp_third_person_game_mode (Utilities|Casting|CastToBP_ThirdPersonGameMode (Game|GetGameMode)))
  (Variables|Default|SetCustomGameMode _asbp_third_person_game_mode))

(event Collision|EventActorBeginOverlap
  (params (OtherActor :type Actor%20Object%20Reference))
  (bind _customgamemode (Variables|Default|GetCustomGameMode))
  ;[1 1 1] Overlap Logic
  (Utilities|IsPlayerCharacter OtherActor
    (:true
      (if (Variables|/Game/ThirdPerson/Blueprints/BP_ThirdPersonGameMode.BP_ThirdPersonGameMode_C|GetGameActive _customgamemode)
        (CallFunction|SpawnStatue)
        ;;[1 0 0.7762] Call OnEventStatueCollected
        (Default|EventStatueCollected _customgamemode)
        (Actor|DestroyActor)))))

(fn ConstructionScript)